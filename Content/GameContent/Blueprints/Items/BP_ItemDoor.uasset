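; BP_ItemDoor is a usable door that opens and closes only when the player has its key.
; OnUse asks the player character whether it holds the Key item, then toggles IsOpen, or prints a debug message if the key is missing.
; ChangeDoorStatus plays a sound and runs a timeline forward or in reverse, feeding its value into the Scene component's yaw to swing the door.
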(event Custom|ChangeDoorStatus
  (Audio|SpawnSoundatLocation "/Game/GameContent/Media/Sounds/OpenDoor.OpenDoor" (Transformation|GetActorLocation) "0, 0, 0" 1.0 1.0 0.0 0 0)
  (if (Variables|Default|GetbIsOpen)
    (bind _alpha (Timeline|Door_TL Play)
      (:Update
        (Transformation|SetRelativeRotation (Variables|Default|GetScene) (Math|Rotator|MakeRotator 0.0 0.0 _alpha) false false)))
    (else
      (Timeline|Door_TL Reverse))))

(fn ConstructionScript
  (|CallParentFunction))

(fn OnUse
  (bind _havekey (CallFunction|HaveKey?))
  (if _havekey
    (Variables|Default|SetbIsOpen (not (Variables|Default|GetbIsOpen)))
    (CallFunction|ChangeDoorStatus)
    (else
      (Development|PrintString "You need the key!"))))

(fn HaveKey?
  (bind _asbp_character_player (Utilities|Casting|CastToBP_CharacterPlayer (Game|GetPlayerCharacter 0)))
  (bind _bexists (Default|HasItem _asbp_character_player (LocalVariables|GetKey)))
  (return _bexists))