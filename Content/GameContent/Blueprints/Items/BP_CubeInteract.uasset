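; BP_CubeInteract is an interactable item Blueprint that triggers an animation on a referenced character when used.
; OnUse checks that CharacterReference is valid, then plays the looping Walking animation directly on that character's skeletal mesh component.
; Without a valid reference, it prints a Spanish debug message saying the character reference does not exist.
; The event graph and construction script add no logic of their own.
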(event EventBeginPlay
  (|CallParentFunction) ; This node is disabled and will not be called.\nDrag off pins to build functionality.
)

(event Collision|EventActorBeginOverlap
  (params (OtherActor :type Actor%20Object%20Reference))
  (|CallParentFunction OtherActor) ; This node is disabled and will not be called.\nDrag off pins to build functionality.
)

(event EventTick
  (params (DeltaSeconds :type Float%20%28single-precision%29))
  (|CallParentFunction DeltaSeconds) ; This node is disabled and will not be called.\nDrag off pins to build functionality.
)

(fn ConstructionScript
  (|CallParentFunction))

(fn OnUse
  (Utilities|IsValid (Variables|Default|GetCharacter_Reference)
    (:Is%20Valid
      (Components|Animation|PlayAnimation (Variables|/Script/Engine.SkeletalMeshActor|GetSkeletalMeshComponent (Variables|Default|GetCharacter_Reference)) "/Game/GameContent/Animations/Walking.Walking" true))
    (:Is%20Not%20Valid
      (Development|PrintString "No existe referencia al character"))))