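; Player Blueprint that lets the player use items in front of them.
; Pressing Use runs a line trace between two GetPlayerLocation points at near and far distances, drawn briefly for debugging, and calls OnUse on any BP_ItemBase it hits.
; GetPlayerLocation contains math for offsetting the actor location along control-rotation forward, though those nodes are marked unused.
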(event Input|ActionEvents|InputActionUse
  (params (Key :type Key%20Structure :default "None"))
  (:Pressed
    (bind (_outhit _returnvalue) (Collision|LineTraceByChannel (Utilities|GetPlayerLocation 4.0) (Utilities|GetPlayerLocation 4e+02) "TraceTypeQuery3" false 0 "ForDuration" true "(R=1.000000,G=0.000000,B=0.000000,A=1.000000)" "(R=0.000000,G=1.000000,B=0.000000,A=1.000000)" 3.0))
    (if _returnvalue
      (bind _asbp_item_base (Utilities|Casting|CastToBP_ItemBase (.HitActor (Collision|BreakHitResult _outhit))))
      (Default|OnUse _asbp_item_base))))

(fn ConstructionScript)